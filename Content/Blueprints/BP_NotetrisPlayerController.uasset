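; Player controller for Notetris that handles pausing and resuming the game.
; The PauseGame input action calls TogglePause, which branches on the current paused state.
; Pausing creates a PauseScreen widget, focuses it in Game and UI input mode, and shows the cursor.
; Resuming removes all widgets from the viewport, restores game-only input, and hides the cursor.
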(event Input|ActionEvents|InputActionPauseGame
  (params (Key :type Key%20Structure :default "None"))
  (:Pressed
    (CallFunction|TogglePause)))

(fn ConstructionScript)

(fn TogglePause
  (bind _returnvalue (Game|GetPlayerController 0))
  (if (Game|IsGamePaused)
    (Game|SetGamePaused false)
    (Viewport|RemoveAllWidgets)
    (Input|SetInputModeGameOnly _returnvalue)
    (Variables|Default|SetbShowMouseCursor false)
    (else
      (Game|SetGamePaused true)
      (bind _returnvalue_2 (UserInterface|CreateWidget "/Game/Assets/UI/PauseScreen.PauseScreen_C" _returnvalue))
      (UserInterface|Viewport|AddtoViewport _returnvalue_2 0)
      (Input|SetInputModeGameandUI _returnvalue _returnvalue_2 "DoNotLock" false)
      (Variables|Default|SetbShowMouseCursor true))))